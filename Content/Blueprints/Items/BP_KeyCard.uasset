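; BP_KeyCard is a keycard pickup that comes in red, orange or blue, selected by its Keycard enum.
; The construction script sets the matching Paper2D sprite, and Tick turns it on yaw toward the player as a billboard.
; When BP_FirstPersonCharacter overlaps the Box, the card sets that color's flag on the character, notifies the player HUD and destroys itself.
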(event OnComponentBeginOverlap(Box)
  (params (OverlappedComponent :type Primitive%20Component%20Object%20Reference) (OtherActor :type Actor%20Object%20Reference) (OtherComp :type Primitive%20Component%20Object%20Reference) (OtherBodyIndex :type Integer) (bFromSweep :type Boolean) (SweepResult :type Hit%20Result%20Structure%20%28by%20ref%29))
  (bind _asbp_first_person_character (Utilities|Casting|CastToBP_FirstPersonCharacter OtherActor))
  (Variables|Default|SetFirstPersonCharacterRef _asbp_first_person_character)
  (switch Utilities|FlowControl|Switch|SwitchonKeyCard (Variables|Default|GetKeycard)
    (:NewEnumerator0
      (Variables|/Game/FirstPerson/Blueprints/BP_FirstPersonCharacter.BP_FirstPersonCharacter_C|SetRedKeyCard? (Variables|Default|GetFirstPersonCharacterRef) true)
      (Default|FindRedKeyCard (Variables|/Game/FirstPerson/Blueprints/BP_FirstPersonCharacter.BP_FirstPersonCharacter_C|GetPlayerHud (Variables|Default|GetFirstPersonCharacterRef))))
    (:NewEnumerator1
      (Variables|/Game/FirstPerson/Blueprints/BP_FirstPersonCharacter.BP_FirstPersonCharacter_C|SetOrangeKeyCard? (Variables|Default|GetFirstPersonCharacterRef) true)
      (Default|FindOrangeKeyCard (Variables|/Game/FirstPerson/Blueprints/BP_FirstPersonCharacter.BP_FirstPersonCharacter_C|GetPlayerHud (Variables|Default|GetFirstPersonCharacterRef))))
    (:NewEnumerator2
      (Variables|/Game/FirstPerson/Blueprints/BP_FirstPersonCharacter.BP_FirstPersonCharacter_C|SetBlueKeyCard? (Variables|Default|GetFirstPersonCharacterRef) true)
      (Default|FindBlueKeyCard (Variables|/Game/FirstPerson/Blueprints/BP_FirstPersonCharacter.BP_FirstPersonCharacter_C|GetPlayerHud (Variables|Default|GetFirstPersonCharacterRef)))))
  (Actor|DestroyActor))

(event EventBeginPlay)

(event Collision|EventActorBeginOverlap
  (params (OtherActor :type Actor%20Object%20Reference)))

(event EventTick
  (params (DeltaSeconds :type Float%20%28single-precision%29))
  (Transformation|SetActorRotation (Math|Rotator|MakeRotator 0.0 0.0 (.yaw (Math|Rotator|FindLookatRotation (Transformation|GetActorLocation) (Transformation|GetActorLocation (Game|GetPlayerCharacter 0)))))))

(fn ConstructionScript
  (switch Utilities|FlowControl|Switch|SwitchonKeyCard (Variables|Default|GetKeycard)
    (:NewEnumerator0
      (Rendering|Components|Sprite|SetSprite (Variables|Default|GetPaperSprite) "/Game/Sprites/Items/redkey_Sprite.redkey_Sprite"))
    (:NewEnumerator1
      (Rendering|Components|Sprite|SetSprite (Variables|Default|GetPaperSprite) "/Game/Sprites/Items/orangekey_Sprite.orangekey_Sprite"))
    (:NewEnumerator2
      (Rendering|Components|Sprite|SetSprite (Variables|Default|GetPaperSprite) "/Game/Sprites/Items/bluekey_Sprite.bluekey_Sprite"))))