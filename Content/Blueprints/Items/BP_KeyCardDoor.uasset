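; Color-coded key card door that opens for a first-person character holding the matching card.
; The KeyCardDoor enum sets the cube's red, orange or blue material in the construction script.
; On box overlap, the same enum picks which character key flag to check.
; A match plays a one-time timeline that raises the cube relative to its current height each update, then destroys the actor after a short delay.
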(event OnComponentBeginOverlap(Box)
  (params (OverlappedComponent :type Primitive%20Component%20Object%20Reference) (OtherActor :type Actor%20Object%20Reference) (OtherComp :type Primitive%20Component%20Object%20Reference) (OtherBodyIndex :type Integer) (bFromSweep :type Boolean) (SweepResult :type Hit%20Result%20Structure%20%28by%20ref%29))
  (bind _cube (Variables|Default|GetCube))
  (bind _returnvalue (Transformation|GetWorldLocation _cube))
  (bind _asbp_first_person_character (Utilities|Casting|CastToBP_FirstPersonCharacter OtherActor))
  (Variables|Default|SetAs%20BP%20First%20Person%20Character _asbp_first_person_character)
  (switch Utilities|FlowControl|Switch|SwitchonKeyCard (Variables|Default|GetKeyCardDoor)
    (:NewEnumerator0
      (if (Variables|/Game/FirstPerson/Blueprints/BP_FirstPersonCharacter.BP_FirstPersonCharacter_C|GetRedKeyCard? (Variables|Default|GetAs%20BP%20First%20Person%20Character))
        (Utilities|FlowControl|DoOnce false :!label _label
          (:Completed
            (bind _newtrack_0 (Timeline|Timeline Play)
              (:Update
                (Transformation|SetWorldLocation _cube (Math|Vector|MakeVector (.x _returnvalue) (.y _returnvalue) (Math|Float|Lerp (.z _returnvalue) (+ (.z _returnvalue) 15.0) _newtrack_0)) false false))
              (:Finished
                (Utilities|FlowControl|Delay 0.2)
                (Actor|DestroyActor)))))))
    (:NewEnumerator1
      (if (Variables|/Game/FirstPerson/Blueprints/BP_FirstPersonCharacter.BP_FirstPersonCharacter_C|GetOrangeKeyCard? (Variables|Default|GetAs%20BP%20First%20Person%20Character))
        (goto _label)))
    (:NewEnumerator2
      (if (Variables|/Game/FirstPerson/Blueprints/BP_FirstPersonCharacter.BP_FirstPersonCharacter_C|GetBlueKeyCard? (Variables|Default|GetAs%20BP%20First%20Person%20Character))
        (goto _label)))))

(event EventBeginPlay)

(event Collision|EventActorBeginOverlap
  (params (OtherActor :type Actor%20Object%20Reference)))

(event EventTick
  (params (DeltaSeconds :type Float%20%28single-precision%29)))

(fn ConstructionScript
  (switch Utilities|FlowControl|Switch|SwitchonKeyCard (Variables|Default|GetKeyCardDoor)
    (:NewEnumerator0
      (Rendering|Material|SetMaterial (Variables|Default|GetCube) 0 "/Game/Sprites/Items/reddoor_Mat.reddoor_Mat"))
    (:NewEnumerator1
      (Rendering|Material|SetMaterial (Variables|Default|GetCube) 0 "/Game/Sprites/Items/Orangedoor_Mat.Orangedoor_Mat"))
    (:NewEnumerator2
      (Rendering|Material|SetMaterial (Variables|Default|GetCube) 0 "/Game/Sprites/Items/bluedoor_Mat.bluedoor_Mat"))))