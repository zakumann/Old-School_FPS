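; Base enemy character drawn as a Doom-style directional Paper2D sprite, with sight, melee and projectile attacks, health and death.
; Each tick it derives an idle, moving or attack state, then uses dot products against the player to pick one of eight flipbooks and its rotation.
; Pawn sensing and damage set CanSeePlayer on the AI blackboard, making it face the player.
; Death stops the brain, plays a death flipbook, leaves a corpse, then destroys it.
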(event OnSeePawn(PawnSensing)
  (params (Pawn :type Pawn%20Object%20Reference))
  ;[1 1 1] HandleEnemyVision
  (Utilities|Casting|CastToBP_FirstPersonCharacter Pawn)
  (Variables|Donotedit|Setcanseeplayer true)
  (AI|Components|Blackboard|SetValueasBool (AI|GetBlackboard 0) (Utilities|Name|MakeLiteralName "CanSeePlayer") true)
  (Utilities|FlowControl|RetriggerableDelay 0.7)
  (Variables|Donotedit|Setcanseeplayer false)
  (AI|Components|Blackboard|SetValueasBool (AI|GetBlackboard 0) (Utilities|Name|MakeLiteralName "CanSeePlayer") false))

(event Custom|RotateTowardsPlayer
  ;[1 1 1] HandleEnemyRotation
  (Transformation|SetActorRotation (Math|Interpolation|RInterpTo (Transformation|GetActorRotation) (Math|Rotator|FindLookatRotation (Transformation|GetActorLocation) (Transformation|GetActorLocation (Game|GetPlayerCharacter 0))) (Utilities|Time|GetWorldDeltaSeconds) (Variables|Edit|GetRotationspeed))))

(event Custom|SpawnProjectile
  ;[1 1 1] AttackSystem
  ;;[1 0 0] RangedAttack
  (Variables|Donotedit|Setisattacking true)
  (Variables|Donotedit|Setattackstate "NewEnumerator1")
  (Components|Movement|StopMovementImmediately (Variables|Character|GetCharacterMovement))
  (Game|SpawnActorfromClass (Variables|Edit|GetEnemyProjectile) (Transformation|GetWorldTransform (Variables|Default|GetProjectileSpawn)) "Undefined" "MultiplyWithRoot" 0 (Variables|Edit|GetProjectile%20Speed) (Variables|Edit|GetProjectile%20Damage) 0)
  (Utilities|FlowControl|RetriggerableDelay (+ (Variables|Edit|GetFireRate) 0.1))
  (Variables|Donotedit|Setisattacking false))

(event Custom|MeleeAttack
  (bind _returnvalue (Transformation|GetActorLocation))
  ;[1 1 1] AttackSystem
  ;;[1 0 0] MeleeAttack
  (Variables|Donotedit|Setisattacking true)
  (Variables|Donotedit|Setattackstate "NewEnumerator0")
  (bind _outhit (Collision|LineTraceForObjects _returnvalue (+ _returnvalue (* (Transformation|GetActorForwardVector) 1.5e+02)) (Utilities|Array|MakeArray "ObjectTypeQuery3") false (Utilities|Array|MakeArray self) "None"))
  (if (== (.HitActor (Collision|BreakHitResult _outhit)) (Game|GetPlayerCharacter 0))
    (Game|Damage|ApplyDamage (.HitActor (Collision|BreakHitResult _outhit)) (Variables|Edit|GetEnemyDamage) 0 0)
    (Utilities|FlowControl|RetriggerableDelay (+ (Variables|Edit|GetMeleeRate) 0.1)))
  (Variables|Donotedit|Setisattacking false))

(event Custom|Handle%20Death
  (bind _paperflipbook (Variables|Default|GetPaperFlipbook))
  ;[1 1 1] HandleEnemyDeathSystem
  (Transformation|SetActorRotation (Math|Rotator|MakeRotator 0.0 0.0 (.yaw (Math|Rotator|FindLookatRotation (Transformation|GetActorLocation) (Transformation|GetActorLocation (Game|GetPlayerCharacter 0))))))
  (Utilities|FlowControl|DoOnce false
    (:Completed
      (AI|Logic|StopLogic (Variables|/Script/AIModule.AIController|GetBrainComponent (AI|GetAIController self)) "isdead")
      (Pawn|Components|CharacterMovement|SetMovementMode (Variables|Character|GetCharacterMovement) "MOVE_Flying" 0)
      (Collision|SetCollisionEnabled (Variables|Default|GetCapsuleComponent) "NoCollision")
      (Components|Activation|Deactivate (Variables|Character|GetCharacterMovement))
      (Transformation|SetRelativeRotation _paperflipbook "0.000000,-90.000000,0.000000" false false)
      (Sprite|SetFlipbook _paperflipbook (Variables|Flipbooks|GetEnemyDeathFlipbook))
      (Utilities|FlowControl|Delay (- (Class|PaperFlipbookComponent|GetFlipbookLength (Variables|Default|GetPaperFlipbook)) 0.2))
      (Transformation|AddActorLocalOffset "0.000000,0.000000,-30.000000" false false)
      (Sprite|SetFlipbook (Variables|Default|GetPaperFlipbook) (Variables|Flipbooks|GetEnemyBodyFlipbook))
      (Utilities|FlowControl|Delay 4.0)
      (Actor|DestroyActor))))

(event EventTick
  (params (DeltaSeconds :type Float%20%28single-precision%29))
  (bind _returnvalue (|HandleEnemystate+CalculateEnemydegree))
  (|SetEnemyRotation+Flipbook _returnvalue))

(event Game|Damage|EventAnyDamage
  (params (Damage :type Float%20%28single-precision%29) (DamageType :type Damage%20Type%20Object%20Reference) (InstigatedBy :type Controller%20Object%20Reference) (DamageCauser :type Actor%20Object%20Reference))
  ;[1 1 1] HandleEnemyDamage
  (bind _output_get (Variables|Edit|Sethealth (- (Variables|Edit|Gethealth) Damage)))
  (if (<= _output_get 0.0)
    (Variables|Donotedit|Setisdead true)
    (else
      (Variables|Donotedit|Setcanseeplayer true)
      (AI|Components|Blackboard|SetValueasBool (AI|GetBlackboard 0) (Utilities|Name|MakeLiteralName "CanSeePlayer") true))))

(fn ConstructionScript)